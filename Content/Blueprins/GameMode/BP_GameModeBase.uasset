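; Game mode base that runs endless waves of aliens, each wave's size scaled by a difficulty multiplier.
; After a short delay it starts a wave, then a looping timer spawns BP_Alien actors at random TargetPoints until the wave's quota is used up.
; Living aliens are tracked in an array; RegisterAlienDeath removes them and, once none remain alive or pending, schedules the next wave after a delay.
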(event `self.ReceiveBeginPlay`
  (`KismetSystemLibrary.Delay` 2.0)
  (`self.SetupNewWave`))

(event `SpawnWave`
  (`self.SpawnAlien`))

(event `EndWave`
  (`KismetSystemLibrary.Delay` 2.0)
  (`self.SetupNewWave`))

(fn `GetRandomSpawnPoint`
  (returns (Output :type "TargetPoint Object Reference"))
  (bind _outactors (`GameplayStatics.GetAllActorsOfClass` "/Script/Engine.TargetPoint"))
  (return (`|GetArrayItem` _outactors (`KismetMathLibrary.RandomIntegerInRange` 0 (`KismetArrayLibrary.Array_LastIndex` _outactors)))))

(fn `Increase Wave Difficulty`
  (bind _output_get (set `self.WaveDiffculty` (`KismetMathLibrary.Round` (* (`self.WaveDiffculty`) (`self.DifficultyMultyplay`)))))
  (set `self.AlienSpawnRemeining` _output_get))

(fn `IsWaveComplite`
  (returns (ReturnValue :type Boolean))
  (return (and (== (`KismetArrayLibrary.Array_Length` (`self.Aliens`)) 0) (== (`self.AlienSpawnRemeining`) 0))))

(fn `RegisterAlienDeath`
  (params (Alien :type "/Game/Characters/Enemy_Great_Spider/AI/BP_Alien Object Reference (by ref)"))
  (`KismetArrayLibrary.Array_RemoveItem` (`self.Aliens`) Alien)
  (if (`self.IsWaveComplite`)
    (`self.EndWave`)))

(fn `SetupNewWave`
  (`/Engine/EditorBlueprintResources/StandardMacros.IncrementInt` (`self.CurrentWave`)
    (:`  `
      (`self.Increase Wave Difficulty`)
      (`KismetSystemLibrary.K2_SetTimer` null "SpawnWave" (`self.Time`) true))))

(fn `SpawnAlien`
  (bind _output (`self.GetRandomSpawnPoint`))
  (`/Engine/EditorBlueprintResources/StandardMacros.IsValid` _output
    (:`Is Valid`
      (bind _returnvalue (`|SpawnActorFromClass` "/Game/Characters/Enemy_Great_Spider/AI/BP_Alien.BP_Alien_C" (`self.GetTransform` _output) "AlwaysSpawn" "OverrideRootScale" null null))
      (`/Engine/EditorBlueprintResources/StandardMacros.IsValid` _returnvalue
        (:`Is Valid`
          (`KismetArrayLibrary.Array_Add` (`self.Aliens`) _returnvalue)
          (bind _result (`/Engine/EditorBlueprintResources/StandardMacros.DecrementInt` (`self.AlienSpawnRemeining`))
            (:`  `
              (if (== _result 0)
                (`KismetSystemLibrary.K2_ClearTimer` null "SpawnWave")))))))))

(fn `UserConstructionScript`)