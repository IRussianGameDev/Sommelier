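; Player character for a twin-stick style shooter, with world-axis movement, sprint, HUD, health, death and kill count.
; Each tick sets control rotation from thumbstick direction or smoothed mouse velocity, both deadzone-filtered, switching on the last key's device.
; Firing runs a looping timer that line-traces from the muzzle along control rotation, applying damage and impact effects.
; Damage clamps health to MaxHealth and stops fire at zero, while healing hard-codes a 100 cap.
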(event `self.ReceiveBeginPlay`
  ;[1 1 1] Event BeginPlay
  (bind _returnvalue (`|CreateWidget` "/Game/UI/W_PlayerHUD.W_PlayerHUD_C" null self))
  (`UserWidget.AddToViewport` _returnvalue 0)
  (set `self.Health` (`self.MaxHealth`)))

(event `InputAction|Sprint`
  (params (Key :type "Key Structure"))
  (:`Pressed`
    (`self.Sprint`))
  (:`Released`
    (`self.Run`)))

(event `InputAction|Fire Weapone`
  (params (Key :type "Key Structure"))
  ;[1 1 1] FireStart/Stop
  (:`Pressed`
    (`self.StartFiringWeapone`))
  (:`Released`
    (`self.StopFiringWeapone`)))

(event `InputAxis|MoveForvard`
  (params (AxisValue :type "Float (single-precision)"))
  ;[1 1 1] Move
  (if (`self.IsAlive`)
    (`self.AddMovementInput` (1.0 0.0 0.0) AxisValue)))

(event `self.ReceiveTick`
  (params (DeltaSeconds :type "Float (single-precision)"))
  ;[1 1 1] Mouse Thumbsick Move
  (`self.UpdatePlayerAim`))

(event `Key|AnyKey`
  (params (Key :type "Key Structure"))
  ;[1 1 1] Mouse Thumbsick Move
  (:`Pressed`
    (set `self.GamepadeActive` (`KismetInputLibrary.Key_IsGamepadKey` Key))))

(event `InputAxis|MoveRight`
  (params (AxisValue :type "Float (single-precision)"))
  ;[1 1 1] Move
  (if (`self.IsAlive`)
    (`self.AddMovementInput` (0.0 1.0 0.0) AxisValue)))

(event `self.ReceiveAnyDamage`
  (params (Damage :type "Float (single-precision)") (DamageType :type "DamageType Object Reference") (InstigatedBy :type "Controller Object Reference") (DamageCauser :type "Actor Object Reference"))
  ;[1 0.1888 0.1749] AnyDamage
  (if (`self.IsAlive`)
    (bind _output_get (`self.DecreaseHealth` Damage))
    (if (== _output_get 0.0)
      (set `self.IsDead` true)
      (`self.StopFiringWeapone`))))

(fn `AddHealth`
  (params (`Health to Add` :type "Float (double-precision)"))
  (set `self.Health` (`KismetMathLibrary.FClamp` (+ (`self.Health`) `Health to Add`) 0.0 100.0)))

(fn `DecreaseHealth`
  (params (Damage :type "Float (double-precision)"))
  (returns (Output_Get :type "Float (double-precision)"))
  (bind _output_get (set `self.Health` (`KismetMathLibrary.FClamp` (- (`self.Health`) Damage) 0.0 (`self.MaxHealth`))))
  (return _output_get))

(fn `GetMouseAimDirection`
  (returns (ReturnValue :type "Rotator Structure"))
  (bind (_returnvalue_x _returnvalue_y) (`KismetMathLibrary.BreakVector2D` (`self.GetMouseVelocity`)))
  (return (`KismetMathLibrary.RInterpTo` (`Controller.GetControlRotation` (`GameplayStatics.GetPlayerController` 0)) (`KismetMathLibrary.MakeRotator` 0.0 0.0 (`KismetMathLibrary.DegAtan2` _returnvalue_x _returnvalue_y)) (`GameplayStatics.GetWorldDeltaSeconds`) (`self.MouseSmoothingStrenght`))))

(fn `GetMouseVelocity`
  (returns (ReturnValue :type "Vector2D Structure"))
  (bind (_deltax _deltay) (`PlayerController.GetInputMouseDelta` (`GameplayStatics.GetPlayerController` 0)))
  (return (/ (`KismetMathLibrary.MakeVector2D` _deltax _deltay) (`GameplayStatics.GetWorldDeltaSeconds`))))

(fn `GetThumvstickDirection`
  (returns (ReturnValue :type "Rotator Structure"))
  (return (`KismetMathLibrary.MakeRotator` 0.0 0.0 (`KismetMathLibrary.DegAtan2` (`self.GetInputAxisValue`) (`self.GetInputAxisValue`)))))

(fn `GetWeaponeTraceEndLocation`
  (returns (ReturnValue :type "Vector Structure"))
  (return (+ (`self.GetWeaponeTraceStartLocation`) (* (`KismetMathLibrary.GetForwardVector` (`self.GetControlRotation`)) (`self.WeaponeRange`)))))

(fn `GetWeaponeTraceStartLocation`
  (returns (ReturnValue :type "Vector Structure"))
  (return (`SceneComponent.GetSocketLocation` (`self.Weapone`) "MuzzleFlashSocket")))

(fn `IncreaseKill`
  (`/Engine/EditorBlueprintResources/StandardMacros.IncrementInt` (`self.Kill`)))

(fn `IsAlive`
  (returns (ReturnValue :type Boolean))
  (return (not (`self.IsDead`))))

(fn `IsHealthFull`
  (returns (ReturnValue :type Boolean))
  (return (== (`self.Health`) 100.0)))

(fn `IsMouseAboveDeadZone`
  (returns (ReturnValue :type Boolean))
  (return (> (`KismetMathLibrary.VSize2D` (`self.GetMouseVelocity`)) (`self.MouseDeadzone`))))

(fn `IsThumStickAboveDeadZone`
  (returns (ReturnValue :type Boolean))
  (return (> (`KismetMathLibrary.VSize2D` (`KismetMathLibrary.MakeVector2D` (`self.GetInputAxisValue`) (`self.GetInputAxisValue`))) (`self.ThumbstickDeadzone`))))

(fn `Run`
  (set `CharacterMovementComponent.MaxWalkSpeed` (`self.NormalSpeed`) (`self.CharacterMovement`))
  (set `self.IsSprinting` false))

(fn `Spawn Impact Hit`
  (params (HitLocation :type "Vector Structure"))
  (`GameplayStatics.SpawnEmitterAtLocation` "/Game/Effects/Weapons/Impacts/P_AssaultRifle_IH.P_AssaultRifle_IH" HitLocation))

(fn `Sprint`
  (set `CharacterMovementComponent.MaxWalkSpeed` (`self.SprintSpeed`) (`self.CharacterMovement`))
  (set `self.IsSprinting` true))

(fn `StartFiringWeapone`
  (if (`self.IsAlive`)
    (`ActorComponent.Activate` (`self.ParticleSystem`) false)
    (bind _returnvalue (`GameplayStatics.SpawnSound2D` "/Game/Sounds/Weapon_AssaultRifle/Stereo/RifleFireLoop_Cue.RifleFireLoop_Cue" 1.0 1.0 0.0 null))
    (set `self.WeaponeSound` _returnvalue)
    (`self.WeaponeTrace`)
    (`KismetSystemLibrary.K2_SetTimer` null "WeaponeTrace" (`self.WeaponeRate`) true)))

(fn `StopFiringWeapone`
  (bind _weaponesound (`self.WeaponeSound`))
  (`ActorComponent.Deactivate` (`self.ParticleSystem`))
  (`/Engine/EditorBlueprintResources/StandardMacros.IsValid` _weaponesound
    (:`Is Valid`
      (`AudioComponent.Stop` _weaponesound)
      (`KismetSystemLibrary.K2_ClearTimer` null "WeaponeTrace")
      (if (`self.IsAlive`)
        (`GameplayStatics.SpawnSound2D` "/Game/Sounds/Weapon_AssaultRifle/Stereo/RifleFireStop_Cue.RifleFireStop_Cue" 1.0 1.0 0.0 null)))))

(fn `UpdateMouseAim`
  (if (`self.IsMouseAboveDeadZone`)
    (`Controller.SetControlRotation` (`GameplayStatics.GetPlayerController` 0) (`self.GetMouseAimDirection`))))

(fn `UpdatePlayerAim`
  (if (`self.IsAlive`)
    (if (`self.GamepadeActive`)
      (`self.UpdateThumbstickAim`)
      (else
        (`self.UpdateMouseAim`)))))

(fn `UpdateThumbstickAim`
  (if (`self.IsThumStickAboveDeadZone`)
    (`Controller.SetControlRotation` (`GameplayStatics.GetPlayerController` 0) (`self.GetThumvstickDirection`))))

(fn `UserConstructionScript`)

(fn `WeaponeTrace`
  (bind _outhit (`KismetSystemLibrary.LineTraceSingle` (`self.GetWeaponeTraceStartLocation`) (`self.GetWeaponeTraceEndLocation`) "TraceTypeQuery1"))
  (bind (_bblockinghit _binitialoverlap _time _distance _location _impactpoint _normal _impactnormal _physmat _hitactor) (`GameplayStatics.BreakHitResult` _outhit))
  (if _bblockinghit
    (`GameplayStatics.ApplyDamage` _hitactor (`self.Base Damage`))
    (`self.Spawn Impact Hit` _location)))