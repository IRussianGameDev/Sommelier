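; BP_Alien is an enemy AI character that chases the player and attacks in melee range.
; A looping AIMoveTo drives pursuit, while Tick checks range and montage state, pausing movement during the attack montage.
; A separate function applies damage to the player but is not called within this Blueprint.
; At zero health it disables movement and collision, credits the player's kill, notifies the game mode, then destroys itself after a delay.
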(event `self.ReceiveBeginPlay`
  (set `self.Health` (`self.MaxHealth`))
  (if (`self.IsAlive`) :!label _label
    (`|AIMoveTo` self (0.0 0.0 0.0) (`GameplayStatics.GetPlayerCharacter` 0)
      (:`OnSuccess`
        _)
      (:`OnFail`
        _))
    (`KismetSystemLibrary.Delay` 0.2)
    (goto _label)))

(event `self.ReceiveTick`
  (params (DeltaSeconds :type "Float (single-precision)"))
  ;[1 1 1] Attack
  (if (`self.CanAttack`)
    (`self.DeactivateAiMovement`)
    (`|PlayMontage` (`self.Mesh`) "/Game/Characters/Enemy_Great_Spider/Animations/AM_AlienAttaco.AM_AlienAttaco"
      (:`OnCompleted`
        (`self.ActivateAIMovement`)))))

(event `self.ReceiveAnyDamage`
  (params (Damage :type "Float (single-precision)") (DamageType :type "DamageType Object Reference") (InstigatedBy :type "Controller Object Reference") (DamageCauser :type "Actor Object Reference"))
  (if (`self.IsAlive`)
    (bind _output_get (`self.DecreaseHealth` Damage))
    (if (== _output_get 0.0)
      (`self.KillAi`)
      (`KismetSystemLibrary.Delay` 3.0)
      (`self.K2_DestroyActor`))))

(fn `ActivateAIMovement`
  (`ActorComponent.Activate` (`self.CharacterMovement`) false))

(fn `CanAttack`
  (returns (ReturnValue :type Boolean))
  (return (and (`self.IsWithinAttackRange`) (not (`self.IsAttacing`)) (`self.IsAlive`))))

(fn `DeactivateAiMovement`
  (bind _charactermovement (`self.CharacterMovement`))
  (`MovementComponent.StopMovementImmediately` _charactermovement)
  (`ActorComponent.Deactivate` _charactermovement))

(fn `DecreaseHealth`
  (params (Damage :type "Float (double-precision)"))
  (returns (Output_Get :type "Float (double-precision)"))
  (bind _output_get (set `self.Health` (`KismetMathLibrary.FClamp` (- (`self.Health`) Damage) 0.0 (`self.MaxHealth`))))
  (return _output_get))

(fn `Dmamge Player`
  (if (`self.IsAlive`)
    (`GameplayStatics.ApplyDamage` (`GameplayStatics.GetPlayerCharacter` 0) (`self.Base Damage`))))

(fn `IsAlive`
  (returns (ReturnValue :type Boolean))
  (return (not (`self.IsDead`))))

(fn `IsAttacing`
  (returns (ReturnValue :type Boolean))
  (if (not (`self.IsDead`))
    (return (`AnimInstance.Montage_IsPlaying` (`SkeletalMeshComponent.GetAnimInstance` (`self.Mesh`)) "/Game/Characters/Enemy_Great_Spider/Animations/AM_AlienAttaco.AM_AlienAttaco"))))

(fn `IsWithinAttackRange`
  (returns (ReturnValue :type Boolean))
  (return (< (`self.GetDistanceTo` (`GameplayStatics.GetPlayerCharacter` 0)) (`self.AttackRange`))))

(fn `KillAi`
  (set `self.IsDead` true)
  (`self.DeactivateAiMovement` self)
  (`self.SetActorEnableCollision` false)
  (bind _asbp_player_character (cast `/Game/Blueprins/Pawns/BP_PlayerCharacter` (`GameplayStatics.GetPlayerCharacter` 0)))
  (set `self.As BP Player Character` _asbp_player_character)
  (`/Game/Blueprins/Pawns/BP_PlayerCharacter.IncreaseKill` (`self.As BP Player Character`))
  (bind _asbp_game_mode_base (cast `/Game/Blueprins/GameMode/BP_GameModeBase` (`GameplayStatics.GetGameMode`)))
  (set `self.As BP Game Mode Base` _asbp_game_mode_base)
  (`/Game/Blueprins/GameMode/BP_GameModeBase.RegisterAlienDeath` (`self.As BP Game Mode Base`) self))

(fn `UserConstructionScript`)